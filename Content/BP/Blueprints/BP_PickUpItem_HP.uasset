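; Health pickup item that restores a fixed amount of HP to the player character.
; Its PickUp event casts the first player pawn to BP_Character and adds to current HP only when it is below max.
; The item destroys itself after healing and stays in place at full health.
; The addition is not clamped, so HP can end above the maximum.
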(event EventPickUp
  (bind _asbp_character (Utilities|Casting|CastToBP_Character (Game|Player|GetPlayerPawn 0)))
  (if (< (Variables|/Game/BP/Blueprints/BP_Character.BP_Character_C|GetHPcurrent_player _asbp_character) (Variables|/Game/BP/Blueprints/BP_Character.BP_Character_C|GetHPmax_player _asbp_character))
    (Variables|/Game/BP/Blueprints/BP_Character.BP_Character_C|SetHPcurrent_player _asbp_character (+ (Variables|/Game/BP/Blueprints/BP_Character.BP_Character_C|GetHPcurrent_player _asbp_character) 5.0))
    (Actor|DestroyActor)))

(fn ConstructionScript
  (|CallParentFunction))