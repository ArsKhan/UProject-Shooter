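; Test turret actor that turns toward the player and fires bullets.
; Each tick it smoothly rotates its Cube toward the player pawn and line-traces from the Cube to the player's location offset by the turret's forward vector.
; A BP_Character hit starts, via a resettable DoOnce, a looping timer spawning scaled-down BP_Basic_Bullet actors at the Arrow.
; Losing the target only resets the DoOnce, never clearing the timer.
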(event Custom|shoot
  (bind _arrow (Variables|Default|GetArrow))
  (bind _returnvalue (Transformation|GetWorldTransform _arrow))
  (Game|SpawnActorfromClass "/Game/BP/Blueprints/BP_Basic_Bullet.BP_Basic_Bullet_C" (Math|Transform|MakeTransform (.location _returnvalue) (.rotation _returnvalue) "0.300000,0.300000,0.300000") "AlwaysSpawn" 0 0))

(event EventTick
  (params (DeltaSeconds :type Float%20%28single-precision%29))
  (bind _returnvalue (Game|Player|GetPlayerPawn 0))
  (bind _cube (Variables|Default|GetCube))
  (bind _cube_2 (Variables|Default|GetCube))
  (bind _returnvalue_2 (Transformation|GetActorLocation _returnvalue))
  (bind _returnvalue_3 (Transformation|GetWorldLocation _cube_2))
  (bind _returnvalue_4 (Math|Rotator|FindLookatRotation _returnvalue_3 _returnvalue_2))
  (bind (_roll _pitch _yaw) (Math|Rotator|BreakRotator _returnvalue_4))
  (bind _outhit (Collision|LineTraceByChannel (Transformation|GetWorldLocation (Variables|Default|GetCube)) (+ (Transformation|GetActorLocation _returnvalue) (* (Transformation|GetActorForwardVector) 1e+04)) "TraceTypeQuery2" true 0 "ForOneFrame"))
  (Transformation|SetWorldRotation _cube (Math|Interpolation|RInterpTo (Transformation|GetWorldRotation _cube) (Math|Rotator|MakeRotator 0.0 _pitch _yaw) (Variables|Default|GetDelta%20time) (Variables|Default|GetRotation%20Speed)) false false)
  (bind _output_get (Variables|Default|SetTarg (.HitActor (Collision|BreakHitResult _outhit))))
  (Utilities|Casting|CastToBP_Character _output_get
    (:then
      (Utilities|FlowControl|DoOnce false :!label _label
        (:Completed
          (Utilities|Time|SetTimerbyEvent (delegate Custom|shoot) 0.6 true 0.5))))
    (:CastFailed
      (goto _label Reset))))

(fn ConstructionScript)